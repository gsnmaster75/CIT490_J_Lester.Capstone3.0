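; An interactable button that pitches a linked actor, ObjectToMove, between two wall angles.
; A box overlap with ThirdPersonCharacter opens a gate for the Interact input and closes it on exit, though input stays enabled.
; Each press runs a button timeline, then a FlipFlop alternately plays or reverses the wall rotation timeline.
; The button's transform comes from MoveButton, and its press offset is zero, so it stays still.
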(event `InputAction|Interact`
  (params (Key :type "Key Structure"))
  (bind _move_button_location (`KismetMathLibrary.BreakTransform` (`self.Move Button`)))
  (:`Pressed`
    (`/Engine/EditorBlueprintResources/StandardMacros.Gate` true :!label _label
      (:`Exit`
        (bind (_direction _buttonin) (`Timeline|Button In` :!via `PlayFromStart`)
          (:`Update`
            (`SceneComponent.K2_SetRelativeLocation` (`self.Button`) (`KismetMathLibrary.VLerp` _move_button_location (- _move_button_location (0.0 0.0 0.0)) _buttonin) false false))
          (:`Finished`
            (`/Engine/EditorBlueprintResources/StandardMacros.FlipFlop`
              (:`A`
                (bind (_direction_2 _wall_track) (`Timeline|Wall Timeline` :!label _label_2)
                  (:`Update`
                    (`self.K2_SetActorRelativeRotation` (`self.objectToMove`) (`KismetMathLibrary.MakeRotator` 0.0 (`KismetMathLibrary.Lerp` (`self.Higher Wall`) (`self.Lower Wall`) _wall_track)) false false))))
              (:`B`
                (goto _label_2 :!via `Reverse`)))))))))

(event `self.Box.OnComponentBeginOverlap`
  (params (OverlappedComponent :type "PrimitiveComponent Object Reference") (OtherActor :type "Actor Object Reference") (OtherComp :type "PrimitiveComponent Object Reference") (OtherBodyIndex :type Integer) (bFromSweep :type Boolean) (SweepResult :type "HitResult Structure (by ref)"))
  (cast `/Game/ThirdPersonBP/Blueprints/ThirdPersonCharacter` OtherActor)
  (`self.EnableInput` (`GameplayStatics.GetPlayerController` 0))
  (goto _label :!via `Open`))

(event `self.Box.OnComponentEndOverlap`
  (params (OverlappedComponent :type "PrimitiveComponent Object Reference") (OtherActor :type "Actor Object Reference") (OtherComp :type "PrimitiveComponent Object Reference") (OtherBodyIndex :type Integer))
  (cast `/Game/ThirdPersonBP/Blueprints/ThirdPersonCharacter` OtherActor)
  (`self.EnableInput` (`GameplayStatics.GetPlayerController` 0))
  (goto _label :!via `Close`))

(fn `UserConstructionScript`
  (`SceneComponent.K2_SetRelativeTransform` (`self.Button`) (`self.Move Button`) false false))